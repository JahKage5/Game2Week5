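; BP_GhostBridgeBase is a bridge base that switches a cube between a pass-through state and a solid one.
; BeginPlay saves the cube's material and collision object type, then calls BridgeToOriginal with no material.
; BridgeToOriginal applies the passed material and disables collision.
; BridgeToNew ignores its material input, restoring the saved material and enabling query and physics collision.
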(event Custom|BridgeToNew
  (params (Material :type Material%20Interface%20Object%20Reference))
  (Rendering|Material|SetMaterial (Variables|Default|GetCube) 0 (Variables|Default|GetOriginal%20Mat))
  (Collision|SetCollisionEnabled (Variables|Default|GetCube) "QueryAndPhysics"))

(event Custom|BridgeToOriginal
  (params (Material :type Material%20Interface%20Object%20Reference))
  (Rendering|Material|SetMaterial (Variables|Default|GetCube) 0 Material)
  (Collision|SetCollisionEnabled (Variables|Default|GetCube) "NoCollision"))

(event EventBeginPlay
  (bind _cube (Variables|Default|GetCube))
  ;[0.15 0.15 0.15 0.5] saves orginal
  (Variables|Default|SetOriginal%20Mat (Rendering|Material|GetMaterial _cube 0))
  (Variables|Default|SetNewVar (Collision|GetCollisionObjectType _cube))
  (CallFunction|BridgetoOriginal))

(fn ConstructionScript)