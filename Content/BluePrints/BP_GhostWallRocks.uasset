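; BP_GhostWallRocks is a rock wall actor that can switch between a solid state and a passable ghost state.
; On BeginPlay it caches the mesh component's original material and its collision object type, though the latter is never used here.
; ChangeToNew applies a supplied material and disables collision.
; ChangeToOriginal restores the cached material and sets collision to query and physics, with both events left for external callers to trigger.
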(event Custom|ChangeToNew
  (params (Material :type Material%20Interface%20Object%20Reference))
  (Rendering|Material|SetMaterial (Variables|Default|Getoaksoaksosaos) 0 Material)
  (Collision|SetCollisionEnabled (Variables|Default|Getoaksoaksosaos) "NoCollision"))

(event Custom|ChangeToOriginal
  (Rendering|Material|SetMaterial (Variables|Default|Getoaksoaksosaos) 0 (Variables|Default|GetOriginal%20Mat))
  (Collision|SetCollisionEnabled (Variables|Default|Getoaksoaksosaos) "QueryAndPhysics"))

(event EventBeginPlay
  ;[0.15 0.15 0.15 0.5] saves orginal
  (Variables|Default|SetOriginal%20Mat (Rendering|Material|GetMaterial (Variables|Default|Getoaksoaksosaos) 0))
  (Variables|Default|SetNewVar (Collision|GetCollisionObjectType (Variables|Default|Getoaksoaksosaos))))

(fn ConstructionScript)