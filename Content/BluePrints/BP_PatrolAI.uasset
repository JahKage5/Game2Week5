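; BP_PatrolAI is an enemy pawn that chases the player and calls LoadCheckpoint on the first-person character when its Box overlaps them.
; BeginPlay picks a random walk speed and starts GoToDestination, an AIMoveTo loop on the player that repeats after a short delay, even on failure.
; A GoToPatrolPoint event cycles shuffled PlayerPoint-tagged PlayerStarts, but nothing here calls it.
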(event OnComponentBeginOverlap(Box)
  (params (OverlappedComponent :type Primitive%20Component%20Object%20Reference) (OtherActor :type Actor%20Object%20Reference) (OtherComp :type Primitive%20Component%20Object%20Reference) (OtherBodyIndex :type Integer) (bFromSweep :type Boolean) (SweepResult :type Hit%20Result%20Structure%20%28by%20ref%29))
  (bind _asbp_first_person_character (Utilities|Casting|CastToBP_FirstPersonCharacter OtherActor))
  (Default|LoadCheckpoint _asbp_first_person_character))

(event Custom|GoToPatrolPoint
  (AI|AIMoveTo self (Transformation|GetActorLocation (Utilities|Array|Get(acopy) (stale EventBeginPlay _outactors) (Variables|Default|GetCurrentPlayerPoint))) 0 1e+02 false
    (:OnSuccess
      (Development|PrintString "Arrived at Destination."))
    (:OnFail
      (Development|PrintString "Failed to get to Destination." true true "(R=1.000000,G=0.000000,B=0.118555,A=1.000000)")))
  (bind _result (Math|Integer|IncrementInt (Variables|Default|GetCurrentPlayerPoint))
    (:%20%20
      (if (>= _result (Utilities|Array|Length (stale EventBeginPlay _outactors)))
        (Variables|Default|SetCurrentPlayerPoint 0)
        (Utilities|Array|Shuffle (stale EventBeginPlay _outactors)))
      (Utilities|FlowControl|Delay 1.0)
      (CallFunction|GotoDestination))))

(event Custom|GoToDestination
  (AI|AIMoveTo self "0, 0, 0" (Game|GetPlayerCharacter 0) 2e+01 false
    (:OnSuccess
      (Development|PrintString "Arrived at Destination."))
    (:OnFail
      (Development|PrintString "Failed to get to Destination." true true "(R=1.000000,G=0.000000,B=0.118555,A=1.000000)")))
  (Utilities|FlowControl|Delay 1.0)
  (CallFunction|GotoDestination))

(event EventBeginPlay
  (bind _outactors (Actor|GetAllActorsOfClasswithTag "/Script/Engine.PlayerStart" (Variables|Default|GetPlayerPoint)))
  (Development|PrintString (Utilities|String|Append "There are " (Utilities|String|ToString(Integer) (Utilities|Array|Length _outactors)) "Patrol points."))
  (Utilities|Array|Shuffle _outactors)
  (Variables|/Script/Engine.CharacterMovementComponent|SetMaxWalkSpeed (Variables|Character|GetCharacterMovement) (Math|Conversions|ToFloat(Integer) (* (Math|Random|RandomIntegerinRange 18 24) 25)))
  (CallFunction|GotoDestination))

(fn ConstructionScript)