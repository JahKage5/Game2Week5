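; Manager actor that temporarily ghost-shifts sets of walls and bridges, triggered by debug keys E and F after enabling player input.
; E switches the ObjectsEffected walls to their new state with the M_GoingGhost material, while F switches the Bridge objects, which receive that material on reverting.
; A five-second Delay inside each loop body leads into a second loop that restores the originals.
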(event EventBeginPlay
  (Input|EnableInput (Game|GetPlayerController 0)))

(event Input|ActionEvents|InputActionGhostShift
  (params (Key :type Key%20Structure :default "None")))

(event Input|KeyboardEvents|DebugKeyE
  (params (Key :type Key%20Structure :default "None") (ActionValue :type Input%20Action%20Value%20Structure))
  (:Pressed
    (Development|PrintString "Shifting Walls")
    (for _array_element (Variables|Default|GetObjectsEffected)
      (Default|ChangetoNew _array_element "/Game/Material/M_GoingGhost.M_GoingGhost")
      (Utilities|FlowControl|Delay 5.0)
      (for _array_element_2 (Variables|Default|GetObjectsEffected)
        (Default|ChangetoOriginal _array_element_2)))))

(event Input|KeyboardEvents|DebugKeyF
  (params (Key :type Key%20Structure :default "None") (ActionValue :type Input%20Action%20Value%20Structure))
  (:Pressed
    (Development|PrintString "Shifting Bridges")
    (for _array_element (Variables|Default|GetBridge)
      (Default|BridgetoNew _array_element)
      (Utilities|FlowControl|Delay 5.0)
      (for _array_element_2 (Variables|Default|GetBridge)
        (Default|BridgetoOriginal _array_element_2 "/Game/Material/M_GoingGhost.M_GoingGhost")))))

(fn ConstructionScript)