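; BP_UIPopUpF is a trigger actor that pops up a temporary UI message when the first-person player enters it.
; On overlap with BP_FirstPersonCharacter it creates a UI_TempUI widget, adds it to the viewport and hides it after a fixed delay.
; The widget is only hidden, never removed, and the end-overlap event is empty, with leftover hide logic left unconnected.
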(event EventBeginPlay)

(event Collision|EventActorBeginOverlap
  (params (OtherActor :type Actor%20Object%20Reference))
  (Utilities|Casting|CastToBP_FirstPersonCharacter OtherActor)
  (bind _returnvalue (UserInterface|CreateWidget "/Game/CustomUI/UI_TempUI.UI_TempUI_C" (Game|GetPlayerController 0)))
  (UserInterface|Viewport|AddtoViewport _returnvalue 0)
  (Widget|SetVisibility _returnvalue "Visible")
  (Utilities|FlowControl|Delay 7.0)
  (Widget|SetVisibility _returnvalue "Hidden"))

(event EventTick
  (params (DeltaSeconds :type Float%20%28single-precision%29)))

(event Collision|EventActorEndOverlap
  (params (OtherActor :type Actor%20Object%20Reference)))

(fn ConstructionScript)